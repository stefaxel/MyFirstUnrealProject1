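; BP_Item is an item actor that shows an equip prompt when the third-person character overlaps it.
; On begin overlap it sets the character's IsOverlappingItem flag, creates an EquipItemPromptBP widget, passes it to SetCorrectItemName and adds it to the viewport.
; On end overlap it clears the flag and removes all top-level prompt widgets.
; SetCorrectItemName is empty here, suggesting a hook for child items.
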(event `self.ReceiveActorBeginOverlap`
  (params (OtherActor :type "Actor Object Reference"))
  (bind _asbp_third_person_character (cast `/Game/ThirdPerson/Blueprints/BP_ThirdPersonCharacter` OtherActor))
  (set `MyProjectCharacter.isOverlappingItem` true _asbp_third_person_character)
  (bind _returnvalue (`|CreateWidget` "/Game/GameBlueprints/EquipItemPromptBP.EquipItemPromptBP_C"))
  (`self.SetCorrectItemName` _returnvalue)
  (`UserWidget.AddToViewport` _returnvalue 0))

(event `self.ReceiveActorEndOverlap`
  (params (OtherActor :type "Actor Object Reference"))
  (bind _asbp_third_person_character (cast `/Game/ThirdPerson/Blueprints/BP_ThirdPersonCharacter` OtherActor))
  (set `MyProjectCharacter.isOverlappingItem` false _asbp_third_person_character)
  (bind _foundwidgets (`WidgetBlueprintLibrary.GetAllWidgetsOfClass` "/Game/GameBlueprints/EquipItemPromptBP.EquipItemPromptBP_C"))
  (for _array_element _foundwidgets
    (`Widget.RemoveFromParent` _array_element)))

(fn `SetCorrectItemName`
  (params (`Widget Reference` :type "/Game/GameBlueprints/EquipItemPromptBP Object Reference")))

(fn `UserConstructionScript`)